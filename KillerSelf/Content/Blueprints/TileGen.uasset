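; TileGen is an unfinished Blueprint that appears intended to spawn tiles in random order.
; BeginPlay only loops while TileNumArray is empty, clearing it each pass without adding entries.
; Disconnected nodes sketch removing a random tile number and spawning a random class from TileActorArray through TileNumArray, but none of them run.
; The construction script is empty.
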(event `self.ReceiveBeginPlay`
  (while (== (`KismetArrayLibrary.Array_Length` (stale _output_get)) 0)
    (bind _output_get (set `self.tileNumArray` _))))

(fn `UserConstructionScript`)